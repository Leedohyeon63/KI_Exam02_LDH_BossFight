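; BP_Silkdash is a dash attack actor that moves player 0 forward and damages enemies of type BP_Sinner that it overlaps.
; On BeginPlay a timeline scales DashSpeed by its float track, stepping the pawn along its forward vector without sweep and placing this actor one step ahead.
; A Delay on the timeline update destroys the actor 0.3 seconds after the dash starts.
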(event `self.ReceiveBeginPlay`
  (bind _returnvalue (`GameplayStatics.GetPlayerPawn` 0))
  (bind (_direction `_새_트랙_0`) (`Timeline|타임라인` :!via `PlayFromStart`)
    (:`Update`
      (bind _returnvalue_2 (+ (`self.K2_GetActorLocation` _returnvalue) (* (`self.GetActorForwardVector` _returnvalue) (* (`self.dashSpeed`) `_새_트랙_0`))))
      (`self.K2_SetActorLocation` _returnvalue _returnvalue_2 false false)
      (`self.K2_SetActorLocation` _returnvalue_2)
      (`KismetSystemLibrary.Delay` 0.3)
      (`self.K2_DestroyActor`))))

(event `self.ReceiveActorBeginOverlap`
  (params (OtherActor :type "Actor Object Reference"))
  (bind _asbp_sinner (cast `/Game/Sinner/BossAI/BP_Sinner` OtherActor))
  (`GameplayStatics.ApplyDamage` _asbp_sinner (`self.Damge`)))

(fn `UserConstructionScript`)