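; BP_Test4 is a test actor in the BossAI folder that acts as a short-lived moving hazard damaging the player.
; On BeginPlay a timeline drives cumulative, unswept location offsets along positive Y and downward in Z, scaled by its track value.
; The timeline update also triggers a three-second delay before the actor destroys itself.
; Overlapping a Player_HO applies a small fixed amount of damage.
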(event `self.ReceiveBeginPlay`
  (bind (_direction `_새_트랙_0`) (`Timeline|타임라인` :!via `PlayFromStart`)
    (:`Update`
      (bind _returnvalue (* `_새_트랙_0` 100.0))
      (`self.K2_SetActorLocation` (- (`self.K2_GetActorLocation`) (`KismetMathLibrary.MakeVector` 0.0 (* _returnvalue -1.0) _returnvalue)))
      (`KismetSystemLibrary.Delay` 3.0)
      (`self.K2_DestroyActor`))))

(event `self.ReceiveActorBeginOverlap`
  (params (OtherActor :type "Actor Object Reference"))
  (bind _asplayer_ho (cast `/Game/HO/Player_HO` OtherActor))
  (`GameplayStatics.ApplyDamage` _asplayer_ho 1.0))

(fn `UserConstructionScript`)